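; CameraFOVComponent is a component for BP_MainCharacter that varies the camera's field of view with the character's movement speed setting.
; On BeginPlay it caches the owning character and its camera.
; Each tick it normalizes MaxWalkSpeed, rather than actual velocity, between the character's minimum and maximum speeds.
; A float curve remaps that value to blend between MinFOV and MaxFOV, and FInterpTo smooths the camera toward the result.
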(event EventBeginPlay
  (bind _asbp_main_character (Utilities|Casting|CastToBP_MainCharacter (Components|GetOwner)))
  (bind _output_get (Variables|Default|SetCharacter _asbp_main_character))
  (Variables|Default|SetCamera (Variables|/Game/Blueprints/Core/BP_MainCharacter.BP_MainCharacter_C|GetCamera _output_get)))

(event EventTick
  (params (DeltaSeconds :type Float%20%28single-precision%29))
  (bind _character (Variables|Default|GetCharacter))
  (bind _camera (Variables|Default|GetCamera))
  (bind _output_get (Variables|Default|SetTargetFOV (Math|Float|NormalizetoRange (Variables|/Script/Engine.CharacterMovementComponent|GetMaxWalkSpeed (Variables|/Script/Engine.Character|GetCharacterMovement _character)) (Variables|/Game/Blueprints/Core/BP_MainCharacter.BP_MainCharacter_C|GetMinimumSpeed _character) (Variables|/Game/Blueprints/Core/BP_MainCharacter.BP_MainCharacter_C|GetMaximumSpeed _character))))
  (Camera|SetFieldOfView _camera (Math|Interpolation|FInterpTo (Variables|/Script/Engine.CameraComponent|GetFieldOfView _camera) (Math|Float|Lerp (Variables|Default|GetMinFOV) (Variables|Default|GetMaxFOV) (Math|Curves|GetFloatValue (Variables|Default|GetFOVCurve) _output_get)) DeltaSeconds 5.0)))