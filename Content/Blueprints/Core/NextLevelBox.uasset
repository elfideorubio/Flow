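; NextLevelBox is a level-exit trigger that loads the level named by NextLevelName when the main character overlaps its box.
; The overlap stops the player controller's Timer widget, plays its time animation, and saves the time to the game instance for Tutorial Level or Level 01.
; The game instance then runs CheckScore before the level opens.
; A completion sound with slow motion and delay is present but disconnected.
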(event OnComponentBeginOverlap(Box)
  (params (OverlappedComponent :type Primitive%20Component%20Object%20Reference) (OtherActor :type Actor%20Object%20Reference) (OtherComp :type Primitive%20Component%20Object%20Reference) (OtherBodyIndex :type Integer) (bFromSweep :type Boolean) (SweepResult :type Hit%20Result%20Structure%20%28by%20ref%29))
  (Utilities|Casting|CastToBP_MainCharacter OtherActor)
  (bind _aspc (Utilities|Casting|CastToPC (Game|GetPlayerController 0)))
  (Variables|/Game/UI/Timer.Timer_C|SetStopTime (Variables|/Game/Blueprints/Fideo/PC.PC_C|GetTimer _aspc) true)
  (Default|PlayTimeAnimation (Variables|/Game/Blueprints/Fideo/PC.PC_C|GetTimer _aspc))
  (bind _returnvalue (Game|GetCurrentLevelName true))
  (bind _asgi (Utilities|Casting|CastToGI (Game|GetGameInstance)))
  (switch string _returnvalue
    (:Tutorial_level
      (Variables|/Game/Blueprints/Core/GI.GI_C|SetTimeLevel1 _asgi (Variables|/Game/UI/Timer.Timer_C|GetCurrentTime (Variables|/Game/Blueprints/Fideo/PC.PC_C|GetTimer _aspc))))
    (:Level01
      (Variables|/Game/Blueprints/Core/GI.GI_C|SetTimeLevel2 _asgi (Variables|/Game/UI/Timer.Timer_C|GetCurrentTime (Variables|/Game/Blueprints/Fideo/PC.PC_C|GetTimer _aspc)))))
  (Default|CheckScore _asgi)
  (Game|OpenLevel(byName) (Variables|Default|GetNextLevelName)))

(fn ConstructionScript)