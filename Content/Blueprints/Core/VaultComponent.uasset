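; Vault component that lifts BP_MainCharacter onto low obstacles it runs into.
; Capsule hits on near-vertical walls faced while not falling, with max walk speed above a threshold, trigger a downward object trace ahead to find the ledge height.
; Tick then raises the character by VaultForce, snapping to the target height and ending the vault once reached or when the character is not falling.
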(event Custom|OnHitWall
  (params (HitComponent :type Primitive%20Component%20Object%20Reference) (OtherActor :type Actor%20Object%20Reference) (OtherComp :type Primitive%20Component%20Object%20Reference) (NormalImpulse :type Vector) (Hit :type Hit%20Result%20Structure%20%28by%20ref%29))
  (bind _returnvalue (Transformation|GetWorldLocation))
  (bind _normal (Collision|BreakHitResult Hit))
  (bind _character (Variables|Default|GetCharacter))
  (bind _returnvalue_2 (Transformation|GetActorForwardVector _character))
  (bind _returnvalue_3 (Math|Vector|MakeVector (.x _returnvalue_2) (.y _returnvalue_2) 0.0))
  (bind _returnvalue_4 (Math|Vector|Normalize _returnvalue_3))
  (bind _returnvalue_5 (* _returnvalue_4 1e+02))
  (bind _returnvalue_6 (+ _returnvalue _returnvalue_5))
  (if (Math|Boolean|ANDBoolean (not (Variables|Default|GetIsVaulting)) (Math|Float|NearlyEqual(Float) (.Z (Math|Vector|BreakVector _normal)) 0.0 0.01) (< (Math|Vector|DotProduct _normal _returnvalue_4) -0.7) (not (AI|Components|NavMovement|IsFalling (Utilities|GetCharacterMovement))))
    (if (< (Variables|Default|GetMinVaultSpeed) (Variables|/Script/Engine.CharacterMovementComponent|GetMaxWalkSpeed (Utilities|GetCharacterMovement)))
      (bind _outhit (Collision|LineTraceForObjects (+ _returnvalue_6 "0, 0,100.000000") (- _returnvalue_6 "0, 0,200.000000") (Utilities|Array|MakeArray "ObjectTypeQuery1" "ObjectTypeQuery2" "ObjectTypeQuery3") false (Utilities|Array|MakeArray (Variables|Default|GetCharacter)) "Persistent"))
      (if (<= (.Z (Math|Vector|BreakVector (.Location (Collision|BreakHitResult _outhit)))) (.Z (Math|Vector|BreakVector (Transformation|GetWorldLocation))))
        (Variables|Default|SetTargetHeight (+ (.Z (Math|Vector|BreakVector (.Location (Collision|BreakHitResult _outhit)))) (Variables|/Script/Engine.CapsuleComponent|GetCapsuleHalfHeight (Variables|/Script/Engine.Character|GetCapsuleComponent (Variables|Default|GetCharacter)))))
        (Variables|Default|SetIsVaulting true)
        (Variables|/Game/Blueprints/Core/BP_MainCharacter.BP_MainCharacter_C|SetShouldSlowDown (Variables|Default|GetCharacter) false)))))

(event Custom|EndVaulting
  (Variables|Default|SetIsVaulting false))

(event EventBeginPlay
  (bind _asbp_main_character (Utilities|Casting|CastToBP_MainCharacter (Components|GetOwner)))
  (Variables|Default|SetCharacter _asbp_main_character)
  (Variables|Default|SetDefaultGravityScale (Variables|/Script/Engine.CharacterMovementComponent|GetGravityScale (Utilities|GetCharacterMovement)))
  (Collision|BindEventtoOnComponentHit (Variables|/Script/Engine.Character|GetCapsuleComponent (Variables|Default|GetCharacter)) (delegate Custom|OnHitWall)))

(event EventTick
  (params (DeltaSeconds :type Float%20%28single-precision%29))
  (bind _vaultforce (Variables|Default|GetVaultForce))
  (bind _character (Variables|Default|GetCharacter))
  (bind _returnvalue (Transformation|GetActorLocation _character))
  (bind _returnvalue_2 (* DeltaSeconds _vaultforce))
  (bind _returnvalue_3 (+ (.z _returnvalue) _returnvalue_2))
  (if (Variables|Default|GetIsVaulting)
    (if (or (<= (Variables|Default|GetTargetHeight) _returnvalue_3) (not (AI|Components|NavMovement|IsFalling (Utilities|GetCharacterMovement))))
      (Transformation|SetActorLocation _character (Math|Vector|MakeVector (.x _returnvalue) (.y _returnvalue) (Variables|Default|GetTargetHeight)) false false)
      (CallFunction|EndVaulting)
      (Variables|/Game/Blueprints/Core/BP_MainCharacter.BP_MainCharacter_C|SetShouldSlowDown (Variables|Default|GetCharacter) false)
      (else
        (Transformation|SetActorLocation _character (Math|Vector|MakeVector (.x _returnvalue) (.y _returnvalue) _returnvalue_3) false false)))))