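; Parkour component for BP_MainCharacter that adds wall running, wall jumps and camera tilt.
; Airborne capsule hits on vertical walls start a run after facing, speed and multi-height trace checks, redirecting velocity along the wall.
; Tick scales gravity by a curve, interpolates camera roll and ends runs on landing or wall loss.
; Jump launches along the facing direction; the last wall, or any wall after a forced stop, is blocked until landing.
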(event Custom|OnHitWall
  (params (HitComponent :type Primitive%20Component%20Object%20Reference) (OtherActor :type Actor%20Object%20Reference) (OtherComp :type Primitive%20Component%20Object%20Reference) (NormalImpulse :type Vector) (Hit :type Hit%20Result%20Structure%20%28by%20ref%29))
  (bind _normal (Collision|BreakHitResult Hit))
  (bind _character (Variables|Default|GetCharacter))
  (bind _returnvalue (Transformation|GetActorForwardVector _character))
  (bind _returnvalue_2 (Math|Vector|RotateVector _normal "0,90.000000, 0"))
  (if (Math|Boolean|ANDBoolean (not (Variables|Default|GetIsWallRunning)) (not (Variables|Default|GetForcedStop)) (!= OtherComp (Variables|Default|GetLastWallRan)) (AI|Components|NavMovement|IsFalling (Utilities|GetCharacterMovementComponent)))
    (if (Math|Float|NearlyEqual(Float) (.Z (Math|Vector|BreakVector _normal)) 0.0 0.01) ; Check if hit  is vertical
      (if (< (Math|Float|Absolute(Float) (.z _returnvalue)) 0.5) ; Check if the character is looking in the right vertical direction
        (if (> (Math|Vector|DotProduct (Math|Vector|Normalize (Math|Vector|MakeVector (.x (Variables|/Script/Engine.MovementComponent|GetVelocity (Utilities|GetCharacterMovementComponent))) (.y (Variables|/Script/Engine.MovementComponent|GetVelocity (Utilities|GetCharacterMovementComponent))) 0.0)) (Math|Vector|Normalize (Math|Vector|MakeVector (.x _returnvalue) (.y _returnvalue) 0.0))) 0.75) ; Check if velocity and look direction are similar
          (if (> (Math|Vector|VectorLength (Math|Vector|MakeVector (.x (Variables|/Script/Engine.MovementComponent|GetVelocity (Utilities|GetCharacterMovementComponent))) (.y (Variables|/Script/Engine.MovementComponent|GetVelocity (Utilities|GetCharacterMovementComponent))) 0.0)) (Variables|Default|GetMinHorizontalSpeedForWallRun)) ; Check if horizontal speed is sufficient
            (Variables|Default|SetWallNormal _normal)
            (if (CallFunction|CheckValidWalltoRun)
              (Variables|/Script/Engine.MovementComponent|SetVelocity (Utilities|GetCharacterMovementComponent) (* (Math|Vector|RotateVectorAroundAxis (select (> (Math|Vector|DotProduct _returnvalue_2 (Math|Vector|MakeVector (.x (Variables|/Script/Engine.MovementComponent|GetVelocity (Utilities|GetCharacterMovementComponent))) (.y (Variables|/Script/Engine.MovementComponent|GetVelocity (Utilities|GetCharacterMovementComponent))) 0.0)) 0.0) _returnvalue_2 (Math|Vector|RotateVector _normal "0,-90.000000, 0")) (* (Variables|Default|GetWallRunStartAngle) -1.0) (Math|Vector|RotateVector (select (> (Math|Vector|DotProduct _returnvalue_2 (Math|Vector|MakeVector (.x (Variables|/Script/Engine.MovementComponent|GetVelocity (Utilities|GetCharacterMovementComponent))) (.y (Variables|/Script/Engine.MovementComponent|GetVelocity (Utilities|GetCharacterMovementComponent))) 0.0)) 0.0) _returnvalue_2 (Math|Vector|RotateVector _normal "0,-90.000000, 0")) "0,90.000000, 0")) (Variables|Default|GetWallRunStartMaxSpeed)))
              (CallFunction|StartWallRunning (> (Math|Vector|DotProduct _returnvalue_2 (Math|Vector|MakeVector (.x (Variables|/Script/Engine.MovementComponent|GetVelocity (Utilities|GetCharacterMovementComponent))) (.y (Variables|/Script/Engine.MovementComponent|GetVelocity (Utilities|GetCharacterMovementComponent))) 0.0)) 0.0) OtherComp))))))))

(event Custom|MoveForward
  (params (Value :type Float%20%28single-precision%29)))

(event Custom|MoveRight
  (params (Value :type Float%20%28single-precision%29)))

(event Custom|Jump
  (params (Pressed :type Boolean))
  (bind _character (Variables|Default|GetCharacter))
  (bind _returnvalue (Transformation|GetActorForwardVector _character))
  (bind _returnvalue_2 (Math|Vector|MakeVector (.x _returnvalue) (.y _returnvalue) 0.0))
  (bind _returnvalue_3 (Math|Vector|Normalize _returnvalue_2))
  (if Pressed
    (Variables|/Script/Engine.MovementComponent|SetVelocity (Utilities|GetCharacterMovementComponent) (* (Math|Vector|RotateVectorAroundAxis _returnvalue_3 (* (Variables|Default|GetWallJumpHeight) -1.0) (Math|Vector|RotateVector _returnvalue_3 "0,90.000000, 0")) (Variables|Default|GetWallJumpForce)))
    (CallFunction|StopWallRunning)))

(event Custom|StopWallRunning
  (Variables|Default|SetIsWallRunning false)
  (Variables|/Script/Engine.CharacterMovementComponent|SetGravityScale (Utilities|GetCharacterMovementComponent) (Variables|Default|GetDefaultGravityScale))
  (Variables|Default|SetWallRunCounter 0.0)
  (Variables|Default|SetTargetCameraTilt 0.0)
  (Variables|/Game/Blueprints/Core/BP_MainCharacter.BP_MainCharacter_C|SetShouldSlowDown (Variables|Default|GetCharacter) false))

(event Custom|StartWallRunning
  (params (Right :type Boolean) (Wall :type Actor%20Component%20Object%20Reference))
  (bind _wallruncameratilt (Variables|Default|GetWallRunCameraTilt))
  (bind _output_get (Variables|Default|SetRight Right))
  (Variables|Default|SetLastWallRan Wall)
  (Variables|Default|SetIsWallRunning true)
  (Variables|Default|SetTargetCameraTilt (Math|Float|SelectFloat (* _wallruncameratilt -1.0) _wallruncameratilt _output_get))
  (Variables|/Game/Blueprints/Core/BP_MainCharacter.BP_MainCharacter_C|SetShouldSlowDown (Variables|Default|GetCharacter) false))

(event EventBeginPlay
  (bind _asbp_main_character (Utilities|Casting|CastToBP_MainCharacter (Components|GetOwner)))
  (Variables|Default|SetCharacter _asbp_main_character)
  (Variables|Default|SetDefaultGravityScale (Variables|/Script/Engine.CharacterMovementComponent|GetGravityScale (Utilities|GetCharacterMovementComponent)))
  (Collision|BindEventtoOnComponentHit (Utilities|GetCapsuleComponent) (delegate Custom|OnHitWall)))

(event EventTick
  (params (DeltaSeconds :type Float%20%28single-precision%29))
  (bind _character (Variables|Default|GetCharacter))
  (bind _targetcameratilt (Variables|Default|GetTargetCameraTilt))
  (bind _returnvalue (Pawn|GetController _character))
  (bind _returnvalue_2 (Pawn|GetControlRotation _returnvalue :!class /Script/Engine.Controller))
  (bind _returnvalue_3 (- (.roll _returnvalue_2) 3.6e+02))
  (bind _returnvalue_4 (> (.roll _returnvalue_2) 1.8e+02))
  (bind _returnvalue_5 (Math|Float|SelectFloat _returnvalue_3 (.roll _returnvalue_2) _returnvalue_4))
  (Utilities|FlowControl|Sequence
    (:then_0
      (if (Variables|Default|GetIsWallRunning)
        (Utilities|FlowControl|Sequence
          (:then_0
            (bind _output_get (Variables|Default|SetWallRunCounter (+ DeltaSeconds (Variables|Default|GetWallRunCounter))))
            (Variables|/Script/Engine.CharacterMovementComponent|SetGravityScale (Utilities|GetCharacterMovementComponent) (* (Math|Curves|GetFloatValue (Variables|Default|GetGravityScaleCurve) _output_get) (Variables|Default|GetDefaultGravityScale)))
            (if (not (AI|Components|NavMovement|IsFalling (Utilities|GetCharacterMovementComponent)))
              (CallFunction|StopWallRunning)))
          (:then_1
            (if (not (CallFunction|CheckValidWalltoRun))
              (Variables|Default|SetForcedStop true)
              (CallFunction|StopWallRunning))))))
    (:then_1
      (if (Variables|Default|GetForcedStop)
        (if (not (AI|Components|NavMovement|IsFalling (Utilities|GetCharacterMovementComponent)))
          (Variables|Default|SetForcedStop false))))
    (:then_2
      (if (not (Math|Float|NearlyEqual(Float) _targetcameratilt _returnvalue_5 0.01))
        (Pawn|SetControlRotation _returnvalue (Math|Rotator|MakeRotator (Math|Interpolation|FInterpTo _returnvalue_5 _targetcameratilt DeltaSeconds (Variables|Default|GetCameraTiltSpeed)) (.pitch _returnvalue_2) (.yaw _returnvalue_2)))
        (elif (!= (Variables|Default|GetTargetCameraTilt) (.roll _returnvalue_2))
          (Pawn|SetControlRotation _returnvalue (Math|Rotator|MakeRotator (Variables|Default|GetTargetCameraTilt) (.pitch _returnvalue_2) (.yaw _returnvalue_2))))))
    (:then_3
      (if (and (Utilities|IsValid (Variables|Default|GetLastWallRan)) (not (AI|Components|NavMovement|IsFalling (Utilities|GetCharacterMovementComponent))))
        (Variables|Default|SetLastWallRan 0)))))

(fn CheckValidWalltoRun
  (bind _character (Variables|Default|GetCharacter))
  (bind _returnvalue (Transformation|GetActorLocation _character))
  (for _array_element (Variables|Default|GetCapsuleCenterWallCheckHeights)
    (bind _returnvalue_2 (Collision|LineTraceForObjects (Math|Vector|MakeVector (.x _returnvalue) (.y _returnvalue) (+ (.z _returnvalue) _array_element)) (+ (Math|Vector|MakeVector (.x _returnvalue) (.y _returnvalue) (+ (.z _returnvalue) _array_element)) (* (* (Variables|Default|GetWallNormal) -1.0) 2e+02)) (Utilities|Array|MakeArray "ObjectTypeQuery1" "ObjectTypeQuery2" "ObjectTypeQuery3") false (Utilities|Array|MakeArray (Variables|Default|GetCharacter)) "None"))
    (if (not _returnvalue_2)
      (return false)))
  (return true))