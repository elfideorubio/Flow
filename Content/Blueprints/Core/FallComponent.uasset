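; Actor component for BP_MainCharacter that applies massive fall damage when the character lands too fast.
; Each Tick it compares the movement component's falling state with the cached one to detect landing, then caches the current state and velocity.
; On landing, if the last vertical velocity is below FallSpeedMaxZ and CheckAngle passes, it clears ShouldSlowDown, zeroes velocity and applies the damage.
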(event EventBeginPlay
  (bind _asbp_main_character (Utilities|Casting|CastToBP_MainCharacter (Components|GetOwner)))
  (Variables|Default|SetCharacter _asbp_main_character))

(event EventTick
  (params (DeltaSeconds :type Float%20%28single-precision%29))
  (bind _character (Variables|Default|GetCharacter))
  (Utilities|IsValid (Variables|Default|GetCharacter)
    (:Is%20Valid
      (Utilities|FlowControl|Sequence
        (:then_0
          (if (Math|Boolean|NotEqual(Boolean) (Variables|Default|GetLastIsFalling) (AI|Components|NavMovement|IsFalling (Variables|/Script/Engine.Character|GetCharacterMovement (Variables|Default|GetCharacter))))
            (if (Variables|Default|GetLastIsFalling)
              (if (and (> (Variables|Default|GetFallSpeedMaxZ) (.z (Variables|Default|GetLastVelocity))) (> (Default|CheckAngle (Variables|Default|GetCharacter)) -1.0))
                (Variables|/Game/Blueprints/Core/BP_MainCharacter.BP_MainCharacter_C|SetShouldSlowDown _character false)
                (Variables|/Script/Engine.MovementComponent|SetVelocity (Variables|/Script/Engine.Character|GetCharacterMovement _character) "0, 0, 0")
                (Game|Damage|ApplyDamage _character 1e+04 0 0)))))
        (:then_1
          (Variables|Default|SetLastIsFalling (AI|Components|NavMovement|IsFalling (Variables|/Script/Engine.Character|GetCharacterMovement (Variables|Default|GetCharacter))))
          (Variables|Default|SetLastVelocity (Variables|/Script/Engine.MovementComponent|GetVelocity (Variables|/Script/Engine.Character|GetCharacterMovement (Variables|Default|GetCharacter)))))))))