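; Game Instance that persists a fastest-time leaderboard for Tutorial Level and Level 01 through an SG_SaveGameInfo save slot.
; SaveGameCheck loads the slot or creates it if missing.
; CheckScore picks the current level's time by map name, inserts it before the first equal or slower entry, drops the last entry, flags that level's record and saves.
; AddPlayerName fills blank-named entries, and ResetRecords clears the record flags.
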(event Custom|SaveGameCheck
  (bind _returnvalue (SaveGame|DoesSaveGameExist (Variables|Default|GetSlotName)))
  (if _returnvalue
    (CallFunction|LoadGame)
    (else
      (CallFunction|SaveGame))))

(event Custom|CheckScore
  (bind _levelname (Variables|Default|GetLevelName))
  (bind _savegamedata (Variables|Default|GetSaveGameData))
  (bind _topscores (Variables|/Game/Blueprints/Fideo/Saving/SG_SaveGameInfo.SG_SaveGameInfo_C|GetTopScores _savegamedata))
  (bind (_topscoreindex _newhighscore_) (CallFunction|CheckScores))
  (Variables|Default|SetSlotToScoreIn _topscoreindex)
  (if _newhighscore_
    (switch Utilities|FlowControl|Switch|SwitchonE_LevelName (Variables|Default|GetLevelName)
      (:NewEnumerator0
        (Variables|Default|SetLevel1Record true))
      (:NewEnumerator1
        (Variables|Default|SetLevel2Record true)))
    (Utilities|Array|Insert _topscores (Utilities|Struct|MakeST_ScoreInfo (Variables|Default|GetPlayerName) (Utilities|Select :Index _levelname :NewEnumerator0 "Level 1" :NewEnumerator1 "Level 2") (Utilities|Select :Index _levelname :NewEnumerator0 (Variables|Default|GetTimeLevel1) :NewEnumerator1 (Variables|Default|GetTimeLevel2))) (Variables|Default|GetSlotToScoreIn))
    (Utilities|Array|RemoveIndex _topscores (Utilities|Array|LastIndex _topscores))
    (CallFunction|SaveGame)))

(event Custom|ResetRecords
  (Variables|Default|SetLevel1Record false)
  (Variables|Default|SetLevel2Record false))

(event Custom|AddPlayerName
  (params (PlayerName :type Text))
  (bind _savegamedata (Variables|Default|GetSaveGameData))
  (bind _topscores (Variables|/Game/Blueprints/Fideo/Saving/SG_SaveGameInfo.SG_SaveGameInfo_C|GetTopScores _savegamedata))
  (for (_array_element _array_index) _topscores
    (if (Utilities|Text|TextIsEmpty (.PlayerName (Utilities|Struct|BreakST_ScoreInfo _array_element)))
      (Utilities|Array|SetArrayElem _topscores _array_index (Utilities|Struct|MakeST_ScoreInfo PlayerName (.LevelName (Utilities|Struct|BreakST_ScoreInfo _array_element)) (.PlayerScore (Utilities|Struct|BreakST_ScoreInfo _array_element))))
      (CallFunction|SaveGame))))

(fn LoadGame
  (bind _returnvalue (SaveGame|LoadGamefromSlot (Variables|Default|GetSlotName)))
  (bind _assg_save_game_info (Utilities|Casting|CastToSG_SaveGameInfo _returnvalue))
  (Variables|Default|SetSaveGameData _assg_save_game_info))

(fn SaveGame
  (Variables|Default|GetSaveGameData
    (:then
      _)
    (:else
      (bind _returnvalue (SaveGame|CreateSaveGameObject "/Game/Blueprints/Fideo/Saving/SG_SaveGameInfo.SG_SaveGameInfo_C"))
      (Variables|Default|SetSaveGameData _returnvalue)))
  (SaveGame|SaveGametoSlot (Variables|Default|GetSaveGameData) (Variables|Default|GetSlotName)))

(fn CheckScores
  (bind _savegamedata (Variables|Default|GetSaveGameData))
  (CallFunction|GetLevelEnum)
  (Utilities|IsValid _savegamedata
    (:Is%20Valid
      _)
    (:Is%20Not%20Valid
      (CallFunction|SaveGameCheck)))
  (bind (_array_element _array_index) (Utilities|Array|ForEachLoopwithBreak (Variables|/Game/Blueprints/Fideo/Saving/SG_SaveGameInfo.SG_SaveGameInfo_C|GetTopScores _savegamedata) :!label _label)
    (:LoopBody
      (if (<= (Utilities|Select :Index (Variables|Default|GetLevelName) :NewEnumerator0 (Variables|Default|GetTimeLevel1) :NewEnumerator1 (Variables|Default|GetTimeLevel2)) (.PlayerScore (Utilities|Struct|BreakST_ScoreInfo _array_element)))
        (LocalVariables|SetIsNewScore true)
        (goto _label Break)))
    (:Completed
      (return _array_index (LocalVariables|GetIsNewScore)))))

(fn GetLevelEnum
  (bind _returnvalue (Game|GetCurrentLevelName true))
  (switch string _returnvalue
    (:Tutorial_level
      (Variables|Default|SetLevelName "NewEnumerator0"))
    (:Level01
      (Variables|Default|SetLevelName "NewEnumerator1"))))