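; Player controller Blueprint that toggles which colour of BP_Platform, red or blue, is visible and collidable.
; BeginPlay sorts every platform in the level into red and blue arrays by its IsRedPlatform flag and adds the WBP_Mouse widget to the viewport.
; Right-click alternates through a FlipFlop, blue first, updating the widget colour, disabling one array and enabling the other, with booleans guarding against repeated activation.
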(event EventBeginPlay
  ;[1 1 1] Getting the platforms references
  (Utilities|FlowControl|Sequence
    (:then_0
      (bind _outactors (Actor|GetAllActorsOfClass "/Game/Blueprints/Fideo/BP_Platform.BP_Platform_C"))
      (for _array_element _outactors
        (if (Variables|/Game/Blueprints/Fideo/BP_Platform.BP_Platform_C|GetbIsRedPlatform? _array_element)
          (Utilities|Array|AddUnique (Variables|Default|GetRedPlatforms) _array_element)
          (else
            (Utilities|Array|AddUnique (Variables|Default|GetBluePlatforms) _array_element)))))
    (:then_1
      ;[1 1 1] UI
      (bind _returnvalue (UserInterface|CreateWidget "/Game/Blueprints/Fideo/WBP_Mouse.WBP_Mouse_C"))
      (bind _output_get (Variables|Default|SetWBP_Mouse_Ref _returnvalue))
      (UserInterface|Viewport|AddtoViewport _output_get 0))))

(event EventTick
  (params (DeltaSeconds :type Float%20%28single-precision%29)))

(event Input|MouseEvents|LeftMouseButton
  (params (Key :type Key%20Structure :default "None")))

(event Input|MouseEvents|RightMouseButton
  (params (Key :type Key%20Structure :default "None"))
  (:Pressed
    (Utilities|FlowControl|FlipFlop
      (:A
        (Variables|Default|SetIsRedPressed? false) ; This avoids repressing
        (if (not (Variables|Default|GetIsBluePressed?))
          (Default|MouseColor (Variables|Default|GetWBP_Mouse_Ref) false) ; UI color update
          ;[1 1 1] Removes the old one first
          (for _array_element (Variables|Default|GetRedPlatforms)
            (Default|SetVisibility/Collision _array_element false))
          ;[1 1 1] Enables the newly selected platforms
          (for _array_element_2 (Variables|Default|GetBluePlatforms)
            (Default|SetVisibility/Collision _array_element_2 true)
            (Variables|Default|SetIsBluePressed? true))))
      (:B
        (Variables|Default|SetIsBluePressed? false)
        (if (not (Variables|Default|GetIsRedPressed?))
          (Default|MouseColor (Variables|Default|GetWBP_Mouse_Ref) true)
          (for _array_element_3 (Variables|Default|GetBluePlatforms)
            (Default|SetVisibility/Collision _array_element_3 false))
          (for _array_element_4 (Variables|Default|GetRedPlatforms)
            (Default|SetVisibility/Collision _array_element_4 true)
            (Variables|Default|SetIsRedPressed? true)))))))

(fn ConstructionScript)