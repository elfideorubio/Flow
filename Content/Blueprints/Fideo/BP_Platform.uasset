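; A red or blue platform that toggles between solid and non-collidable, with blue starting without collision.
; The construction script picks the color material, mesh and scale, and sets custom depth stencil 2 for red.
; SetVisibility/Collision plays or reverses a timeline driving that color's shared opacity parameter in MPC_Opacity.
; Showing restores collision and disables custom depth immediately, while hiding does the opposite once the fade finishes.
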(event Custom|SetVisibility/Collision
  (params (Visible? :type Boolean))
  (bind _cube (Variables|Default|GetCube))
  (if Visible?
    (Rendering|SetRenderCustomDepth (Variables|Default|GetCube) false) ; Turn it off because it's visible
    (Collision|SetCollisionEnabled (Variables|Default|GetCube) "QueryAndPhysics")
    (bind _alphafloat (Timeline|Timeline_0 PlayFromStart)
      (:Update
        (Rendering|Material|SetScalarParameterValue "/Game/Materials/Blockout/MPC_Opacity.MPC_Opacity" (select (Variables|Default|GetbIsRedPlatform?) "RedOpacity" "BlueOpacity") (Math|Float|Lerp 0.0 1.0 _alphafloat) :!class /Script/Engine.KismetMaterialLibrary))
      (:Finished
        (if (not Visible?)
          (Rendering|SetRenderCustomDepth _cube true)
          (Collision|SetCollisionEnabled _cube "NoCollision"))))
    (else
      (Timeline|Timeline_0 ReverseFromEnd))))

(event EventBeginPlay)

(fn ConstructionScript
  (bind _cube (Variables|Default|GetCube))
  (Rendering|Material|SetMaterial (Variables|Default|GetCube) 0 (select (Variables|Default|GetbIsRedPlatform?) "/Game/Materials/Environment/MI_PlatformMaterial_Red.MI_PlatformMaterial_Red" "/Game/Materials/Environment/MI_PlatformMaterial_Blue.MI_PlatformMaterial_Blue"))
  (Rendering|Material|SetScalarParameterValue "/Game/Materials/Blockout/MPC_Opacity.MPC_Opacity" "BlueOpacity" 1.0 :!class /Script/Engine.KismetMaterialLibrary)
  (Components|StaticMesh|SetStaticMesh (Variables|Default|GetCube) (Variables|Default|GetStaticMesh))
  (Transformation|SetRelativeScale3D (Variables|Default|GetCube) (Math|Vector|MakeVector (Variables|Default|GetX) (Variables|Default|GetY) (Variables|Default|GetZ)))
  (if (Variables|Default|GetbIsRedPlatform?)
    (Rendering|SetRenderCustomDepth _cube false)
    (Rendering|SetCustomDepthStencilValue _cube 2)
    (else
      ;[1 1 1] Blue collision in the beggining
      (Collision|SetCollisionEnabled (Variables|Default|GetCube) "NoCollision"))))