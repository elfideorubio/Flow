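; Slide component for BP_MainCharacter that crouches, tilts the camera and slides when ground speed exceeds a threshold, otherwise flags a slowdown.
; Sliding zeroes ground friction, sets braking from CheckAngle and launches velocity pitched by that slope angle, with speed scaled by slope.
; Tick retries a held slide request until it succeeds, since falling and wall running block it.
; Stopping uncrouches and restores the friction and braking cached at BeginPlay.
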(event Custom|StopSliding
  (bind _maincharacter (Variables|Default|GetMainCharacter))
  (bind _maincharacter_2 (Variables|Default|GetMainCharacter))
  (bind _charactermovement (Variables|/Script/Engine.Character|GetCharacterMovement _maincharacter_2))
  (Variables|Default|SetWantstoSlide false)
  (if (AI|Components|NavMovement|IsCrouching (Variables|/Script/Engine.Character|GetCharacterMovement (Variables|Default|GetMainCharacter)))
    (Default|EndCameraTilt _maincharacter)
    (Character|UnCrouch _maincharacter)
    (Variables|Default|SetIsSliding false)
    (Variables|/Script/Engine.CharacterMovementComponent|SetGroundFriction _charactermovement (Variables|Default|GetDefaultGroundFriction))
    (Variables|/Script/Engine.CharacterMovementComponent|SetBrakingDecelerationWalking _charactermovement (Variables|Default|GetDefaultBrakingDeceleration))))

(event Custom|StartSliding
  (bind _maincharacter (Variables|Default|GetMainCharacter))
  (bind _maximumslidespeed (Variables|Default|GetMaximumSlideSpeed))
  (bind _maincharacter_2 (Variables|Default|GetMainCharacter))
  (bind _maincharacter_3 (Variables|Default|GetMainCharacter))
  (bind _angle (Default|CheckAngle _maincharacter_2))
  (bind _charactermovement (Variables|/Script/Engine.Character|GetCharacterMovement _maincharacter))
  (bind _returnvalue (> _angle 1.0))
  ;[1 1 1] Sliding
  (Variables|Default|SetWantstoSlide true)
  (if (and (not (AI|Components|NavMovement|IsFalling (Variables|/Script/Engine.Character|GetCharacterMovement _maincharacter_3))) (not (Variables|/Game/Blueprints/Core/ParkourComponent.ParkourComponent_C|GetIsWallRunning (Variables|/Game/Blueprints/Core/BP_MainCharacter.BP_MainCharacter_C|GetParkourComponent _maincharacter_3))))
    (Default|BeginCameraTilt (Variables|Default|GetMainCharacter))
    (Character|Crouch _maincharacter_3)
    (if (< (Variables|Default|GetMinSlideStartSpeed) (Math|Vector|VectorLength (Variables|/Script/Engine.MovementComponent|GetVelocity (Variables|/Script/Engine.Character|GetCharacterMovement (Variables|Default|GetMainCharacter)))))
      (Variables|Default|SetIsSliding true)
      (Variables|/Script/Engine.CharacterMovementComponent|SetGroundFriction _charactermovement 0.0)
      (Variables|/Script/Engine.CharacterMovementComponent|SetBrakingDecelerationWalking _charactermovement (Math|Float|SelectFloat 0.0 256.0 _returnvalue))
      (Variables|/Script/Engine.MovementComponent|SetVelocity _charactermovement (* (Math|Vector|Normalize (Math|Vector|RotateVectorAroundAxis (Math|Vector|MakeVector (.X (Math|Vector|BreakVector (Variables|/Script/Engine.MovementComponent|GetVelocity (Variables|/Script/Engine.Character|GetCharacterMovement (Variables|Default|GetMainCharacter))))) (.Y (Math|Vector|BreakVector (Variables|/Script/Engine.MovementComponent|GetVelocity (Variables|/Script/Engine.Character|GetCharacterMovement (Variables|Default|GetMainCharacter))))) 0.0) (* _angle -1.0) (Math|Vector|RotateVector (Math|Vector|MakeVector (.X (Math|Vector|BreakVector (Variables|/Script/Engine.MovementComponent|GetVelocity (Variables|/Script/Engine.Character|GetCharacterMovement (Variables|Default|GetMainCharacter))))) (.Y (Math|Vector|BreakVector (Variables|/Script/Engine.MovementComponent|GetVelocity (Variables|/Script/Engine.Character|GetCharacterMovement (Variables|Default|GetMainCharacter))))) 0.0) "0,-90.000000,0.000000"))) (Math|Float|SelectFloat (Math|Float|Max(Float) _maximumslidespeed (Math|Vector|VectorLength (Variables|/Script/Engine.MovementComponent|GetVelocity _charactermovement))) (Math|Float|Lerp (Variables|Default|GetMinimumSlideSpeed) _maximumslidespeed (Math|Float|NormalizetoRange _angle -45.0 45.0)) _returnvalue)))
      (else
        (Variables|/Game/Blueprints/Core/BP_MainCharacter.BP_MainCharacter_C|SetShouldSlowDown (Variables|Default|GetMainCharacter) true)))))

(event EventBeginPlay
  (bind _asbp_main_character (Utilities|Casting|CastToBP_MainCharacter (Components|GetOwner)))
  (Variables|Default|SetMainCharacter _asbp_main_character)
  (Variables|Default|SetDefaultGroundFriction (Variables|/Script/Engine.CharacterMovementComponent|GetGroundFriction (Variables|/Script/Engine.Character|GetCharacterMovement (Variables|Default|GetMainCharacter))))
  (Variables|Default|SetDefaultBrakingDeceleration (Variables|/Script/Engine.CharacterMovementComponent|GetBrakingDecelerationWalking (Variables|/Script/Engine.Character|GetCharacterMovement (Variables|Default|GetMainCharacter)))))

(event EventTick
  (params (DeltaSeconds :type Float%20%28single-precision%29))
  (if (Variables|Default|GetWantstoSlide)
    (if (not (Variables|Default|GetIsSliding))
      (Variables|Default|SetWantstoSlide false)
      (CallFunction|StartSliding))))